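; BP_Enemy_Spline is an enemy actor that travels along a level spline path when play begins.
; It finds a BP_SplinePath actor, then plays a timeline at a rate of 1/Duration.
; The timeline's alpha interpolates distance over the spline's length to set the actor's world location each update.
; The spline rotation lookup is left unconnected, so the actor does not orient to the path.
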(event `self.ReceiveBeginPlay`
  (`parent.ReceiveBeginPlay`)
  (bind _returnvalue (`GameplayStatics.GetActorOfClass` "/Game/Blueprints/Spline/BP_SplinePath.BP_SplinePath_C"))
  (set `self.Spline Ref` _returnvalue)
  (`self.MoveTheDummy`))

(event `MoveTheDummy`
  (bind _spline (`/Game/Blueprints/Spline/BP_SplinePath.Spline` (`self.Spline Ref`)))
  (`TimelineComponent.SetPlayRate` (`self.Timeline`) (/ 1.0 (`self.Duration`)))
  (bind (_direction _alpha) (`Timeline|Timeline`)
    (:`Update`
      (`self.K2_SetActorLocationAndRotation` (`SplineComponent.GetLocationAtDistanceAlongSpline` _spline (`KismetMathLibrary.Lerp` 0.0 (`SplineComponent.GetSplineLength` _spline) _alpha) "World")))))

(fn `UserConstructionScript`
  (`parent.UserConstructionScript`))